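; Machine gun weapon Blueprint that fires repeated sci-fi projectiles while the trigger is held.
; Fire opens a Gate that loops through a 0.2-second Delay until Release closes it.
; Each shot plays a sound, decrements ammo and spawns a projectile at an offset aimed by the player's control rotation.
; Ammo is checked only when Fire is called, not inside the loop.
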(event Custom|Release
  (bind _returnvalue (Game|Player|GetPlayerPawn 0))
  (bind _returnvalue_2 (Pawn|GetControlRotation _returnvalue :!class /Script/Engine.Pawn))
  (Utilities|FlowControl|Gate true) ; enters at Close
)

(event Custom|Fire
  (bind _returnvalue (Game|Player|GetPlayerPawn 0))
  (bind _returnvalue_2 (Pawn|GetControlRotation _returnvalue :!class /Script/Engine.Pawn))
  (if (> (Variables|Default|GetAmmoCount) 0)
    (Utilities|FlowControl|Sequence
      (:then_0
        (goto _label Open))
      (:then_1
        (Utilities|FlowControl|Gate true :!label _label
          (:Exit
            (Audio|SpawnSoundAttached "/Game/Audio/SciFiRetriggered.SciFiRetriggered" (VehicleSound|GetRootComponent) "None" "0, 0, 0" "0, 0, 0" "KeepRelativeOffset" false 1.2)
            (Variables|Default|SetAmmoCount (- (Variables|Default|GetAmmoCount) 1))
            (Game|SpawnActorfromClass "/Game/Blueprints/BasicSciFiProjectile.BasicSciFiProjectile_C" (Math|Transform|MakeTransform (+ (Transformation|GetActorLocation) (Math|Vector|RotateVector (Variables|Default|GetGunOffset) _returnvalue_2)) _returnvalue_2) "AlwaysSpawn" 0 0)
            (Utilities|FlowControl|Delay 0.2)
            (goto _label)))))))

(fn ConstructionScript)